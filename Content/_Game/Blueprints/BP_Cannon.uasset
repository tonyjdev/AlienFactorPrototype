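; Player cannon that fires projectiles, takes damage and ends the game when destroyed, with widgets for its input key and health.
; After a random delay at BeginPlay, chained timelines open its doors and move its cylinders out before enabling shooting.
; Health and shots-per-letter live in the GameMode's CannonsArray at ItemIndex, alongside a local shot counter.
; Damage triggers smoke, then fire, then an explosion, after which the fire grows on Tick.
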(event `self.ReceiveTick`
  (params (DeltaSeconds :type "Float (single-precision)"))
  (bind _returnvalue (* DeltaSeconds 1.0))
  (bind _relativescale3d_x (`KismetMathLibrary.BreakVector` (`SceneComponent.RelativeScale3D` (`self.Fire`))))
  (if (`self.IsExploded`)
    (if (< _relativescale3d_x 7.0)
      (`SceneComponent.SetRelativeScale3D` (`self.Fire`) (+ (`SceneComponent.RelativeScale3D` (`self.Fire`)) (`KismetMathLibrary.MakeVector` _returnvalue _returnvalue _returnvalue))))))

(event `FindGameModeRef`
  (bind _output_get (set `self.GameMode_Ref` (cast `/Game/_Game/Blueprints/Core/BP_GameMode` (`GameplayStatics.GetGameMode`) :!pure true) :!label _label))
  (`/Engine/EditorBlueprintResources/StandardMacros.IsValid` _output_get
    (:`Is Not Valid`
      (goto _label))))

(event `self.ReceiveBeginPlay`
  (`self.FindGameModeRef` :!label _label_2)
  (`/Engine/EditorBlueprintResources/StandardMacros.IsValid` (`self.GameMode_Ref`)
    (:`Is Valid`
      (`self.ResetCannon`)
      (`KismetSystemLibrary.Delay` (`KismetMathLibrary.RandomFloatInRange` 0.0 3.0))
      (`self.ActivateCannon`))
    (:`Is Not Valid`
      (goto _label_2))))

(event `ActivateCannon`
  (`TimelineComponent.SetPlayRate` (`self.RotateDoor`) (`self.OpenDoorPlayRate`))
  (`GameplayStatics.PlaySoundAtLocation` "/Game/_Game/Audio/Cues/ElectricDoor-open_Cue.ElectricDoor-open_Cue" (`SceneComponent.K2_GetComponentLocation` (`self.DefaultSceneRoot`)) (struct) 1.0 1.0 0.0 null null null null)
  (bind (_direction _doorrotation) (`Timeline|RotateDoor` :!via `PlayFromStart`)
    (:`Update`
      (`SceneComponent.K2_SetRelativeRotation` (`self.RightDoor`) (`KismetMathLibrary.RLerp` (`self.RightStartRotation`) (`self.RightEndRotation`) _doorrotation) false false)
      (`SceneComponent.K2_SetRelativeRotation` (`self.LeftDoor`) (`KismetMathLibrary.RLerp` (`self.LeftStartRotation`) (`self.LeftEndRotation`) _doorrotation) false false))
    (:`Finished`
      (bind (_direction_2 _cylinderlocation) (`Timeline|ActivateOuterCylinder` :!via `PlayFromStart`)
        (:`Update`
          (`SceneComponent.K2_SetRelativeLocation` (`self.CylinderOuter`) (`KismetMathLibrary.VLerp` (`self.OuterCylinderStartPos`) (`self.OuterCylinderEndPos`) _cylinderlocation) false false)
          (`SceneComponent.K2_SetRelativeLocation` (`self.CylinderInner`) (`KismetMathLibrary.VLerp` (`self.InnerCylinderStartPos`) (`self.InnerCylinderEndPos`) _cylinderlocation) false false))
        (:`Finished`
          (set `self.CanShoot` true))))))

(event `ResetCannon`
  (`SceneComponent.K2_SetRelativeRotation` (`self.RightDoor`) (`self.RightStartRotation`) false false)
  (`SceneComponent.K2_SetRelativeRotation` (`self.LeftDoor`) (`self.LeftStartRotation`) false false)
  (`SceneComponent.K2_SetRelativeLocation` (`self.CylinderOuter`) (`self.OuterCylinderStartPos`) false false)
  (`SceneComponent.K2_SetRelativeLocation` (`self.CylinderInner`) (`self.InnerCylinderStartPos`) false false)
  (`ActorComponent.Deactivate` (`self.Smoke`))
  (`ActorComponent.Deactivate` (`self.Fire`)))

(fn `ApplyDamage`
  (bind _fire (`self.Fire`))
  (bind (_isactive _bp_cannon _inputitem _health _canshoot _shootsperletter) (break `/Game/_Game/Data/STRUCT_Cannon` (`|GetArrayItem` (`/Game/_Game/Blueprints/Core/BP_GameMode.CannonsArray` (`self.GameMode_Ref`)) (`self.ItemIndex`))))
  (bind _returnvalue (`KismetMathLibrary.FClamp` (- _health 0.1)))
  (bind _returnvalue_2 (> _returnvalue 0.0))
  (`KismetArrayLibrary.Array_Set` (`/Game/_Game/Blueprints/Core/BP_GameMode.CannonsArray` (`self.GameMode_Ref`)) (`self.ItemIndex`) (make `/Game/_Game/Data/STRUCT_Cannon` _isactive _bp_cannon _inputitem _returnvalue _returnvalue_2 _shootsperletter))
  (`self.UpdateDamage` false)
  (if (< _returnvalue 0.5)
    (`ActorComponent.Activate` (`self.Smoke`) false)
    (if (< _returnvalue 0.3)
      (if (not (`ActorComponent.IsActive` (`self.Fire`)))
        (`ActorComponent.Activate` _fire false)
        (`GameplayStatics.PlaySoundAtLocation` "/Game/_Game/Audio/Cues/BurningFire_Cue.BurningFire_Cue" (`SceneComponent.K2_GetComponentLocation` _fire) (struct) 1.0 1.0 0.0 null null null null))))
  (if (not _returnvalue_2)
    (`SceneComponent.SetVisibility` (`self.CylinderInner`) false false)
    (`self.Explode`)
    (`/Game/_Game/Blueprints/Core/BP_GameMode.GameOver` (`self.GameMode_Ref`))))

(fn `CheckShootsCounter`
  (returns (Restarted :type Boolean))
  (if (<= (`self.ShootsCounter`) 0)
    (set `self.ShootsCounter` (`self.ShootsPerLetter`))
    (return true)
    (else
      (return false))))

(fn `Explode`
  (bind (_returnvalue_x _returnvalue_y) (`KismetMathLibrary.BreakVector` (`SceneComponent.K2_GetComponentLocation` (`self.Smoke`))))
  (`GameplayStatics.SpawnEmitterAtLocation` "/Game/StarterContent/Particles/P_Explosion.P_Explosion" (`KismetMathLibrary.MakeVector` (+ (`KismetMathLibrary.RandomFloatInRange` -100.0 100.0) _returnvalue_x) (+ (`KismetMathLibrary.RandomFloatInRange` -100.0 100.0) _returnvalue_y) 60.0) (struct) (5.0 5.0 5.0))
  (set `self.IsExploded` true)
  (`GameplayStatics.PlaySoundAtLocation` "/Game/_Game/Audio/Cues/ExplosionPlayer_Cue.ExplosionPlayer_Cue" (`SceneComponent.K2_GetComponentLocation` (`self.DefaultSceneRoot`)) (struct) 1.0 1.0 0.0 null null null null))

(fn `SetHealth`
  (params (NewHealth :type "Float (double-precision)"))
  (bind _returnvalue (`KismetMathLibrary.FClamp` NewHealth))
  (bind (_isactive _bp_cannon _inputitem _health _canshoot _shootsperletter) (break `/Game/_Game/Data/STRUCT_Cannon` (`|GetArrayItem` (`/Game/_Game/Blueprints/Core/BP_GameMode.CannonsArray` (`self.GameMode_Ref`)) (`self.ItemIndex`))))
  (`KismetArrayLibrary.Array_Set` (`/Game/_Game/Blueprints/Core/BP_GameMode.CannonsArray` (`self.GameMode_Ref`)) (`self.ItemIndex`) (make `/Game/_Game/Data/STRUCT_Cannon` _isactive _bp_cannon _inputitem _returnvalue (> _returnvalue 0.0) _shootsperletter))
  (`self.UpdateDamage` false))

(fn `SetShootsPerLetter`
  (params (NewShootsPerLetter :type Integer))
  (bind (_isactive _bp_cannon _inputitem _health _canshoot) (break `/Game/_Game/Data/STRUCT_Cannon` (`|GetArrayItem` (`/Game/_Game/Blueprints/Core/BP_GameMode.CannonsArray` (`self.GameMode_Ref`)) (`self.ItemIndex`))))
  (`KismetArrayLibrary.Array_Set` (`/Game/_Game/Blueprints/Core/BP_GameMode.CannonsArray` (`self.GameMode_Ref`)) (`self.ItemIndex`) (make `/Game/_Game/Data/STRUCT_Cannon` _isactive _bp_cannon _inputitem _health _canshoot NewShootsPerLetter))
  (bind _output_get (set `self.ShootsPerLetter` NewShootsPerLetter))
  (set `self.ShootsCounter` _output_get))

(fn `ShootProjectile`
  (if (`self.CanShoot`)
    (`|SpawnActorFromClass` "/Game/_Game/Blueprints/BP_Projectile.BP_Projectile_C" (`KismetMathLibrary.MakeTransform` (`SceneComponent.K2_GetComponentLocation` (`self.ProjectileSpawner`)) (struct :`Yaw` 180.0)) "Undefined" "OverrideRootScale" null null)
    (`/Engine/EditorBlueprintResources/StandardMacros.DecrementInt` (`self.ShootsCounter`))))

(fn `UpdateDamage`
  (params (ForceUpdate :type Boolean))
  (bind (_isactive _bp_cannon _inputitem _health) (break `/Game/_Game/Data/STRUCT_Cannon` (`|GetArrayItem` (`/Game/_Game/Blueprints/Core/BP_GameMode.CannonsArray` (`self.GameMode_Ref`)) (`self.ItemIndex`))))
  (if ForceUpdate
    (bind _asui_health (cast `/Game/_Game/UI/UI_Health` (`WidgetComponent.GetUserWidgetObject` (`self.Widget_Health`)) :!label _label))
    (`/Game/_Game/UI/UI_Health.UpdateHealth` _asui_health _health)
    (elif _isactive
      (goto _label))))

(fn `UpdateInputItem`
  (params (InputIndex :type Integer))
  (bind _asui_cannon (cast `/Game/_Game/UI/UI_Cannon` (`WidgetComponent.GetUserWidgetObject` (`self.Widget_InputKey`))))
  (`/Game/_Game/UI/UI_Cannon.UpdateInputItemText` _asui_cannon InputIndex))

(fn `UserConstructionScript`)