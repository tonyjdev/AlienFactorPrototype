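; Enemy spaceship that flies along spline paths, damages the cannon on contact and awards score when hit by a projectile.
; BeginPlay scales speed with the GameMode level up to a cap and gathers child splines, occasionally picking a random one for centrally spawned ships, otherwise the first.
; Tick moves the ship by distance along the chosen spline.
; Either hit triggers an explosion effect, sound and destruction.
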(event `self.ReceiveBeginPlay`
  (bind _speed (`self.Speed`))
  ;[1 1 1] Initial Config - Begin Play
  (set `self.IsMoving` true)
  (set `self.IsExploding` false)
  (set `self.Speed` (`KismetMathLibrary.FClamp` (+ (* (`/Game/_Game/Blueprints/Core/BP_GameMode.Level` (cast `/Game/_Game/Blueprints/Core/BP_GameMode` (`GameplayStatics.GetGameMode`) :!pure true)) 10) _speed) 0.0 (+ _speed (`self.MaxAcceleration`))))
  (`KismetArrayLibrary.Array_Clear` (`self.SplineArray`))
  (for _array_element (`SceneComponent.GetChildrenComponents` (`self.DefaultSceneRoot`) false)
    (bind _asspline_component (cast `SplineComponent` _array_element))
    (`KismetArrayLibrary.Array_Add` (`self.SplineArray`) _asspline_component))
  (`self.SelectEnemyPath`))

(event `self.ReceiveTick`
  (params (DeltaSeconds :type "Float (single-precision)"))
  ;[1 1 1] Movement - Tick
  (`self.Moving` DeltaSeconds))

(event `Moving`
  (params (`Delta Seconds` :type "Float (double-precision)"))
  (bind (_returnvalue_location _returnvalue_rotation) (`KismetMathLibrary.BreakTransform` (`SplineComponent.GetTransformAtDistanceAlongSpline` (`|GetArrayItem` (`self.SplineArray`) (`self.SplineIndex`)) (`self.Distance`) "Local" false)))
  ;[1 1 1] Moving Spaceship
  (set `self.Distance` (+ (* `Delta Seconds` (`self.Speed`)) (`self.Distance`)))
  (`SceneComponent.K2_SetRelativeTransform` (`self.Spaceship`) (`KismetMathLibrary.MakeTransform` _returnvalue_location _returnvalue_rotation) false false))

(event `SelectEnemyPath`
  (bind (_returnvalue_x _returnvalue_y) (`KismetMathLibrary.BreakVector` (`SceneComponent.K2_GetComponentLocation` (`self.DefaultSceneRoot`))))
  (if (and (> _returnvalue_y -1000.0) (< _returnvalue_y 1000.0))
    (if (< (`KismetMathLibrary.RandomIntegerInRange` 0 10) 3)
      (bind _output_get (set `self.SplineIndex` (`KismetMathLibrary.RandomIntegerInRange` 0 (- (`KismetArrayLibrary.Array_Length` (`self.SplineArray`)) 1))))
      (`KismetSystemLibrary.PrintString` (`KismetStringLibrary.Conv_IntToString` _output_get))
      (else
        (set `self.SplineIndex` 0 :!label _label)))
    (else
      (goto _label))))

(event `self.Collision.OnComponentBeginOverlap`
  (params (OverlappedComponent :type "PrimitiveComponent Object Reference") (OtherActor :type "Actor Object Reference") (OtherComp :type "PrimitiveComponent Object Reference") (OtherBodyIndex :type Integer) (bFromSweep :type Boolean) (SweepResult :type "HitResult Structure (by ref)"))
  ;[1 1 1] Detect Collision
  (bind _asbp_cannon (cast `/Game/_Game/Blueprints/BP_Cannon` OtherActor)
    (:`then`
      (`/Game/_Game/Blueprints/BP_Cannon.ApplyDamage` _asbp_cannon))
    (:`CastFailed`
      (bind _asbp_projectile (cast `/Game/_Game/Blueprints/BP_Projectile` OtherActor))
      (`self.K2_DestroyActor` _asbp_projectile)
      (`/Game/_Game/Blueprints/Core/BP_GameMode.AddScore` (cast `/Game/_Game/Blueprints/Core/BP_GameMode` (`GameplayStatics.GetGameMode`) :!pure true) (`self.EnemyPoints`))))
  (`self.Explosion`))

(event `Explosion`
  (`GameplayStatics.SpawnEmitterAtLocation` "/Game/StarterContent/Particles/P_Explosion.P_Explosion" (`KismetMathLibrary.MakeVector` (.x (`SceneComponent.K2_GetComponentLocation` (`self.Collision`))) (.y (`SceneComponent.K2_GetComponentLocation` (`self.Collision`))) (+ (.z (`SceneComponent.K2_GetComponentLocation` (`self.Collision`))) 60.0)) (struct) (2.0 2.0 2.0))
  (`GameplayStatics.PlaySoundAtLocation` "/Game/_Game/Audio/Cues/ExplosionEnemy_Cue.ExplosionEnemy_Cue" (`SceneComponent.K2_GetComponentLocation` (`self.DefaultSceneRoot`)) (struct) 1.0 1.0 0.0 null null null null)
  (`self.K2_DestroyActor`))

(fn `UserConstructionScript`)